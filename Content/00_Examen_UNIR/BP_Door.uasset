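; BP_Door is a two-panel sliding door that opens only while every linked button is active.
; On BeginPlay it binds to each ArrayButtons pressed-changed dispatcher, then rechecks all states, acting only when the combined result changes.
; DoorsTimeline plays to open and reverses to close, but its update always lerps from current panel positions toward the open offsets, with no stored closed position.
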(event Custom|CheckButtomStatus
  ;[0.15 0.15 0.15 0.5] Inicializamos el bind a los eventos de los botones, y luego, en función del estado de los botones que hemos configurado chequea los mismos para saber si tiene que abrir o cerrar la puerta
  (Development|PrintString "La puerta reconoce Event Dispacher del FloorButton")
  (Variables|Default|SetInitDoorState (Variables|Default|GetDoorState))
  (Variables|Default|SetDoorState true)
  (for _array_element (Variables|Default|GetarrayButtons)
    (if (not (Variables|/Game/00_Examen_UNIR/BP_FloorButton.BP_FloorButton_C|GetButtonState _array_element))
      (Variables|Default|SetDoorState false)))
  ;;[0.15 0.15 0.15 0.5] Sólo actualiza el estado de la puerta en el caso de que haya cambiado, sino no hace nada.
  (Development|PrintString (Utilities|String|Append "Estado de la puerta tras chequeo: " (Utilities|String|ToString(Boolean) (Variables|Default|GetDoorState))))
  (if (!= (Variables|Default|GetDoorState) (Variables|Default|GetInitDoorState))
    (if (Variables|Default|GetDoorState)
      (if true
        (Development|PrintString "Lanza Apertura Puerta")
        (CallFunction|OpenDoor))
      (elif true
        (Development|PrintString "Lanza Cierre Puerta")
        (CallFunction|CloseDoor)))))

(event Custom|OpenDoor
  ;[0.15 0.15 0.15 0.5] Eventos que gestionan la animación de apertura y cierre de puerta
  (bind _newtrack_0 (Timeline|DoorsTimeline Play)
    (:Update
      (Transformation|SetRelativeLocation (Variables|Default|GetSM_RightDoor) (Math|Vector|Lerp(Vector) (Variables|/Script/Engine.SceneComponent|GetRelativeLocation (Variables|Default|GetSM_RightDoor)) "150.000000,0.000000,0.000000" _newtrack_0) false false)
      (Transformation|SetRelativeLocation (Variables|Default|GetSM_LeftDoor) (Math|Vector|Lerp(Vector) (Variables|/Script/Engine.SceneComponent|GetRelativeLocation (Variables|Default|GetSM_LeftDoor)) "-150.000000,0.000000,0.000000" _newtrack_0) false false))))

(event Custom|CloseDoor
  ;[0.15 0.15 0.15 0.5] Eventos que gestionan la animación de apertura y cierre de puerta
  (bind _newtrack_0 (Timeline|DoorsTimeline Reverse)
    (:Update
      (Transformation|SetRelativeLocation (Variables|Default|GetSM_RightDoor) (Math|Vector|Lerp(Vector) (Variables|/Script/Engine.SceneComponent|GetRelativeLocation (Variables|Default|GetSM_RightDoor)) "150.000000,0.000000,0.000000" _newtrack_0) false false)
      (Transformation|SetRelativeLocation (Variables|Default|GetSM_LeftDoor) (Math|Vector|Lerp(Vector) (Variables|/Script/Engine.SceneComponent|GetRelativeLocation (Variables|Default|GetSM_LeftDoor)) "-150.000000,0.000000,0.000000" _newtrack_0) false false))))

(event EventBeginPlay
  ;[0.15 0.15 0.15 0.5] Inicializamos el bind a los eventos de los botones, y luego, en función del estado de los botones que hemos configurado chequea los mismos para saber si tiene que abrir o cerrar la puerta
  (for _array_element (Variables|Default|GetarrayButtons)
    (EventDispatchers|BindEventtoOnPressedChanged _array_element (delegate Custom|CheckButtomStatus))))

(fn ConstructionScript)