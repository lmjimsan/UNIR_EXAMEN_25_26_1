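; BP_FloorButton is a floor button that the player toggles with the E key.
; Overlap of its sphere by BP_ThirdPersonCharacter enables the actor's input; leaving calls DisableInput on the player controller rather than the button.
; Each press flips ButtonState, swaps the hieroglyph mesh between on and off emissive materials, and fires the OnPressedChanged event dispatcher.
; Debug strings print at each step.
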(event OnComponentBeginOverlap(SphereColl)
  (params (OverlappedComponent :type Primitive%20Component%20Object%20Reference) (OtherActor :type Actor%20Object%20Reference) (OtherComp :type Primitive%20Component%20Object%20Reference) (OtherBodyIndex :type Integer) (bFromSweep :type Boolean) (SweepResult :type Hit%20Result%20Structure%20%28by%20ref%29))
  ;[0.15 0.15 0.15 0.5] Evento que gestiona cuando detecta que entramos en el SphereColl
  (Utilities|Casting|CastToBP_ThirdPersonCharacter OtherActor)
  (Development|PrintString "El Player entró en el botón")
  (Input|EnableInput (Game|GetPlayerController 0)))

(event OnComponentEndOverlap(SphereColl)
  (params (OverlappedComponent :type Primitive%20Component%20Object%20Reference) (OtherActor :type Actor%20Object%20Reference) (OtherComp :type Primitive%20Component%20Object%20Reference) (OtherBodyIndex :type Integer))
  ;[0.15 0.15 0.15 0.5] Evento que gestiona cuando detecta que salimos del SphereColl
  (Utilities|Casting|CastToBP_ThirdPersonCharacter OtherActor)
  (Development|PrintString "El Player salió del botón")
  (Input|DisableInput (Game|GetPlayerController 0) 0))

(event EventBeginPlay
  ;[0.15 0.15 0.15 0.5] Inicializamos las variables: Material de Hieroglyph
  (Rendering|Material|SetMaterial (Variables|Default|GetSM_hieroglyph_007) 0 "/Game/00_Examen_UNIR/M_Emission_btn_off.M_Emission_btn_off"))

(event Input|KeyboardEvents|E
  (params (Key :type Key%20Structure :default "None"))
  ;[0.15 0.15 0.15 0.5] Rutina para cuando se pulse la tecla E y estemos sobre el botón
  (:Pressed
    (Development|PrintString "Presionada la tecla E")
    (bind _output_get (Variables|Default|SetButtonState (not (Variables|Default|GetButtonState))))
    (Development|PrintString (Utilities|String|Append "Estado del botón: " (Utilities|String|ToString(Boolean) _output_get)))
    (if _output_get
      (Rendering|Material|SetMaterial (Variables|Default|GetSM_hieroglyph_007) 0 "/Game/00_Examen_UNIR/M_Emission_btn_on.M_Emission_btn_on")
      (else
        (Rendering|Material|SetMaterial (Variables|Default|GetSM_hieroglyph_007) 0 "/Game/00_Examen_UNIR/M_Emission_btn_off.M_Emission_btn_off")))
    (Development|PrintString "Lanzamos Event Dispacher")
    (Default|CallOnPressedChanged)))

(fn ConstructionScript)